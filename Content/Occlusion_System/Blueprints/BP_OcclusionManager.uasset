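; Occlusion manager Blueprint that produces an occlusion mask from an RGB camera feed and displays it for debugging.
; Each Tick it draws the MT_RGB_feed texture into the RT_CameraInput render target through a canvas, then passes that target to OcclusionInference.
; When the resulting FinalMask is valid, it is set as the image on a WBP_MaskDebug widget added to the viewport at BeginPlay.
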(event `self.ReceiveTick`
  (params (DeltaSeconds :type "Float (single-precision)"))
  (bind _occlusioninference (`self.OcclusionInference`))
  (bind _finalmask (`OcclusionInferenceComponent.FinalMask` _occlusioninference))
  (bind (_canvas _size _context) (`KismetRenderingLibrary.BeginDrawCanvasToRenderTarget` "/Game/Occlusion_System/Materials/RT_CameraInput.RT_CameraInput"))
  (`Canvas.K2_DrawTexture` _canvas "/Game/Media/MT_RGB_feed.MT_RGB_feed" (0.0 0.0) (0.0 0.0) (0.0 0.0) (1.0 1.0) (struct :`R` 1.0 :`G` 1.0 :`B` 1.0 :`A` 1.0) "BLEND_Masked" 0.0 (0.5 0.5))
  (`KismetRenderingLibrary.EndDrawCanvasToRenderTarget` _context)
  (`OcclusionInferenceComponent.RunInference` _occlusioninference "/Game/Occlusion_System/Materials/RT_CameraInput.RT_CameraInput")
  (if (`KismetSystemLibrary.IsValid` _finalmask)
    (`Image.SetBrushFromTexture` (`/Game/Occlusion_System/Widgets/WBP_MaskDebug.DebugImage` (`self.MaskWidget`)) _finalmask false)))

(event `self.ReceiveBeginPlay`
  (bind _returnvalue (`|CreateWidget` "/Game/Occlusion_System/Widgets/WBP_MaskDebug.WBP_MaskDebug_C"))
  (bind _output_get (set `self.MaskWidget` _returnvalue))
  (`UserWidget.AddToViewport` _output_get 0))

(fn `UserConstructionScript`)