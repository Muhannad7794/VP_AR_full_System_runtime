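; Virtual production tracker anchor that uses Live Link to drive a referenced tracked camera with smoothing and a lens offset.
; On each Live Link update, gated by IsLogging, AdaptiveSmoothing filters the camera-role frame.
; The smoothed pose, made relative to the raw pose and composed with LensOffset, becomes the camera's relative transform.
; ApplyLensOffset sets the offset alone; the TRACKDATA CSV-style logging chains are disconnected.
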(event `self.LiveLinkComponentController.OnLiveLinkUpdated`
  (params (DeltaTime :type "Float (single-precision)"))
  (if (`self.IsLogging`)
    (bind _dataresult (`|EvaluateLiveLinkFrameWithSpecificRole` (struct :`Name` "SN30014451") "/Script/LiveLinkInterface.LiveLinkCameraRole")
      (:`then`
        (bind (_staticdata _framedata) (break `LiveLinkCameraBlueprintData` _dataresult))
        (bind (_outsmoothedloc _outsmoothedrot) (`AdaptiveSmoothingComponent.GetSmoothedTransform` (`self.AdaptiveSmoothing`) DeltaTime (`KismetMathLibrary.MakeVector` (.x (.location (`.Transform` (break `LiveLinkCameraFrameData` _framedata)))) (.y (.location (`.Transform` (break `LiveLinkCameraFrameData` _framedata)))) (.z (.location (`.Transform` (break `LiveLinkCameraFrameData` _framedata))))) (`KismetMathLibrary.MakeRotator` (.roll (.rotation (`.Transform` (break `LiveLinkCameraFrameData` _framedata)))) (.pitch (.rotation (`.Transform` (break `LiveLinkCameraFrameData` _framedata)))) (.yaw (.rotation (`.Transform` (break `LiveLinkCameraFrameData` _framedata)))))))
        (`self.K2_SetActorRelativeTransform` (`self.TrackedCameraRefrence`) (`KismetMathLibrary.ComposeTransforms` (`KismetMathLibrary.MakeRelativeTransform` (`KismetMathLibrary.MakeTransform` (`KismetMathLibrary.MakeVector` (.x _outsmoothedloc) (.y _outsmoothedloc) (.z _outsmoothedloc)) (`KismetMathLibrary.MakeRotator` (.roll _outsmoothedrot) (.pitch _outsmoothedrot) (.yaw _outsmoothedrot))) (`KismetMathLibrary.MakeTransform` (`KismetMathLibrary.MakeVector` (.x (.location (`.Transform` (break `LiveLinkCameraFrameData` _framedata)))) (.y (.location (`.Transform` (break `LiveLinkCameraFrameData` _framedata)))) (.z (.location (`.Transform` (break `LiveLinkCameraFrameData` _framedata))))) (`KismetMathLibrary.MakeRotator` (.roll (.rotation (`.Transform` (break `LiveLinkCameraFrameData` _framedata)))) (.pitch (.rotation (`.Transform` (break `LiveLinkCameraFrameData` _framedata)))) (.yaw (.rotation (`.Transform` (break `LiveLinkCameraFrameData` _framedata))))))) (`self.lensOffset`)) false false)))))

(fn `Apply Lens Offset`
  (bind _trackedcamerarefrence (`self.TrackedCameraRefrence`)
    (:`then`
      (`self.K2_SetActorRelativeTransform` _trackedcamerarefrence (`self.lensOffset`) false false))
    (:`else`)))

(fn `UserConstructionScript`)